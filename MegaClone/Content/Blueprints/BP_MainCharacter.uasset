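; BP_MainCharacter is the player character, moving in fixed steps across a small bounded grid in world space.
; Four input actions each offset the capsule component by one cell along X or Y when pressed.
; Each move first checks the actor's world location against the grid bounds, keeping it within a three-by-three area when aligned to the step size.
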(event `self.ReceiveTick`
  (params (DeltaSeconds :type "Float (single-precision)")))

(event `InputAction|MoveRight`
  (params (Key :type "Key Structure"))
  (:`Pressed`
    (if (< (.x (.location (`self.GetTransform`))) 200.0)
      (`SceneComponent.K2_AddWorldOffset` (`self.CapsuleComponent`) (100.0 0.0 0.0) false false))))

(event `InputAction|MoveLeft`
  (params (Key :type "Key Structure"))
  (:`Pressed`
    (if (> (.x (.location (`self.GetTransform`))) 0.0)
      (`SceneComponent.K2_AddWorldOffset` (`self.CapsuleComponent`) (-100.0 0.0 0.0) false false))))

(event `InputAction|MoveUp`
  (params (Key :type "Key Structure"))
  (:`Pressed`
    (if (> (.y (.location (`self.GetTransform`))) 0.0)
      (`SceneComponent.K2_AddWorldOffset` (`self.CapsuleComponent`) (0.0 -100.0 0.0) false false))))

(event `InputAction|MoveDown`
  (params (Key :type "Key Structure"))
  (:`Pressed`
    (if (< (.y (.location (`self.GetTransform`))) 200.0)
      (`SceneComponent.K2_AddWorldOffset` (`self.CapsuleComponent`) (0.0 100.0 0.0) false false))))

(fn `UserConstructionScript`)